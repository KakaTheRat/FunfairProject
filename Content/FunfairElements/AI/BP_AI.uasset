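; BP_AI is a funfair NPC that wanders endlessly between randomly chosen CheckPoint actors in the level.
; It moves with AI MoveTo, notifies each checkpoint it reaches, then recursively picks another, also retrying on failure.
; Each tick it checks distance to the third-person player; when close, it disables movement, turns to face the player and sets NearPlayer, otherwise it restores walking.
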(event `self.ReceiveBeginPlay`
  (bind _outactors (`GameplayStatics.GetAllActorsOfClass` "/Game/FunfairElements/AI/CheckPoint.CheckPoint_C"))
  (set `self.AllCheckPoints` _outactors)
  (`self.MoveToRandomCheckpoint`)
  (bind _returnvalue (`GameplayStatics.GetActorOfClass` "/Game/ThirdPerson/Blueprints/BP_ThirdPersonCharacter.BP_ThirdPersonCharacter_C"))
  (set `self.Player` _returnvalue))

(event `MoveToRandomCheckpoint`
  (bind _output_get (set `self.CurrentCheckpoint` (`KismetArrayLibrary.Array_Random` (`self.AllCheckPoints`))))
  (`|AIMoveTo` self (`SceneComponent.K2_GetComponentLocation` (`/Game/FunfairElements/AI/CheckPoint.Sphere` _output_get)) null 15.0
    (:`OnSuccess`
      (`/Game/FunfairElements/AI/CheckPoint.Reached` _output_get self))
    (:`OnFail`
      _))
  (`self.MoveToRandomCheckpoint`))

(event `self.ReceiveTick`
  (params (DeltaSeconds :type "Float (single-precision)"))
  (bind _capsulecomponent (`self.CapsuleComponent`))
  (bind _charactermovement (`self.CharacterMovement`))
  (if (< (`KismetMathLibrary.Vector_Distance` (`SceneComponent.K2_GetComponentLocation` (`Character.CapsuleComponent` (`self.Player`))) (`SceneComponent.K2_GetComponentLocation` (`self.CapsuleComponent`))) 300.0)
    (`CharacterMovementComponent.DisableMovement` _charactermovement)
    (`SceneComponent.K2_SetWorldRotation` _capsulecomponent (`KismetMathLibrary.FindLookAtRotation` (`SceneComponent.K2_GetComponentLocation` _capsulecomponent) (`SceneComponent.K2_GetComponentLocation` (`Character.CapsuleComponent` (`self.Player`)))) false false)
    (set `self.Near Player` true)
    (else
      (`CharacterMovementComponent.SetMovementMode` _charactermovement "MOVE_Walking" 0)
      (set `self.Near Player` false))))

(fn `UserConstructionScript`)