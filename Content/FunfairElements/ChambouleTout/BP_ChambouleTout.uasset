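; Chamboule-tout funfair minigame actor: overlapping its cylinder starts a can-knockdown game with limited throws, switching the view to the booth.
; ThrowBall spawns a physics ball at the camera and launches it through the deprojected mouse position, randomly offset by the UI's cursor distance.
; Cans leaving CanCheck add score, which decides the win shown when play ends.
; Replay and EndGame destroy balls and restore saved can transforms, toggling physics around the teleport.
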(event `self.ReceiveBeginPlay`
  (`self.CreateUI`)
  (`self.RegisterCan`)
  (`KismetSystemLibrary.PrintString` (`KismetStringLibrary.Concat_StrStr` "Il y a " (`KismetStringLibrary.Conv_IntToString` (`KismetArrayLibrary.Array_Length` (`self.AllCans`))) " cans")))

(event `StartGame`
  (bind _player (`self.Player`))
  (set `self.Throw` 3)
  (`/Game/FunfairElements/ChambouleTout/WB_ChambouleTout.Reset` (`self.UI`))
  (`PlayerController.SetViewTargetWithBlend` (`GameplayStatics.GetPlayerController` 0) self 0.5 "VTBlend_Linear" 0.0 false)
  (`/Game/ThirdPerson/Blueprints/BP_ThirdPersonCharacter.SetVisibility` _player false)
  (`/Game/ThirdPerson/Blueprints/BP_ThirdPersonCharacter.SetStatic` _player true)
  (`/Game/ThirdPerson/Blueprints/BP_ThirdPersonCharacter.SetCrosshairVisibility` _player true)
  (`self.SetUiVisibility` true)
  (set `self.CanThrow` true))

(event `EndGame`
  (bind _player (`self.Player`))
  (bind _returnvalue (`GameplayStatics.GetActorOfClass` "/Game/ThirdPerson/Blueprints/BP_ThirdPersonCharacter.BP_ThirdPersonCharacter_C"))
  (`PlayerController.SetViewTargetWithBlend` (`GameplayStatics.GetPlayerController` 0) _returnvalue 0.5 "VTBlend_Linear" 0.0 false)
  (`/Game/ThirdPerson/Blueprints/BP_ThirdPersonCharacter.SetVisibility` _player true)
  (`/Game/ThirdPerson/Blueprints/BP_ThirdPersonCharacter.SetStatic` _player false)
  (`/Game/ThirdPerson/Blueprints/BP_ThirdPersonCharacter.SetCrosshairVisibility` _player false)
  (`self.SetUiVisibility` false)
  (`self.DestroyBalls`)
  (`self.ResetCanTransform`)
  (set `self.CanThrow` false)
  (set `self.Win` false)
  (set `self.Score` 0))

(event `self.Cylinder.OnComponentBeginOverlap`
  (params (OverlappedComponent :type "PrimitiveComponent Object Reference") (OtherActor :type "Actor Object Reference") (OtherComp :type "PrimitiveComponent Object Reference") (OtherBodyIndex :type Integer) (bFromSweep :type Boolean) (SweepResult :type "HitResult Structure (by ref)"))
  (bind _asbp_third_person_character (cast `/Game/ThirdPerson/Blueprints/BP_ThirdPersonCharacter` OtherActor))
  (set `self.Player` _asbp_third_person_character)
  (`self.StartGame`))

(event `CreateUI`
  (bind _returnvalue (`|CreateWidget` "/Game/FunfairElements/ChambouleTout/WB_ChambouleTout.WB_ChambouleTout_C" (`GameplayStatics.GetPlayerController` 0)))
  (set `self.UI` _returnvalue))

(event `SetUiVisibility`
  (params (Visible :type Boolean))
  (bind _ui (`self.UI`))
  (if Visible
    (`UserWidget.AddToViewport` _ui 0)
    (else
      (`Widget.RemoveFromParent` _ui))))

(event `SaveCanTransform`
  (for _array_element (`self.AllCans`)
    (`KismetArrayLibrary.Array_Add` (`self.CanTransform`) (`SceneComponent.K2_GetComponentToWorld` _array_element))))

(event `ResetCanTransform`
  (for (_array_element _array_index) (`self.AllCans`)
    (bind _asprimitive_component (cast `PrimitiveComponent` _array_element)
      (:`then`
        (`PrimitiveComponent.SetSimulatePhysics` _asprimitive_component false)
        (`SceneComponent.K2_SetWorldTransform` _array_element (`|GetArrayItem` (`self.CanTransform`) _array_index) false true)
        (`PrimitiveComponent.SetSimulatePhysics` _asprimitive_component true))
      (:`CastFailed`
        (`KismetSystemLibrary.PrintString` "Cast Failed")))))

(event `RegisterCan`
  (set `self.AllCans` (`self.GetCans`))
  (`self.SaveCanTransform`))

(event `DestroyBalls`
  (bind _outactors (`GameplayStatics.GetAllActorsOfClass` "/Game/FunfairElements/ChambouleTout/BP_Ball.BP_Ball_C"))
  (for _array_element _outactors
    (`self.K2_DestroyActor` _array_element)))

(event `ThrowBall`
  (bind _cursordist (`/Game/FunfairElements/ChambouleTout/WB_ChambouleTout.CursorDist` (`self.UI`)))
  (if (`self.CanThrow`)
    (set `self.CanThrow` false)
    (set `self.MiniGameTime` false)
    (`/Game/FunfairElements/ChambouleTout/WB_ChambouleTout.PauseAnim` (`self.UI`))
    (bind _returnvalue (`|SpawnActorFromClass` "/Game/FunfairElements/ChambouleTout/BP_Ball.BP_Ball_C" (`SceneComponent.K2_GetComponentToWorld` (`self.Camera`)) "Undefined" "MultiplyWithRoot" null null))
    (bind _returnvalue_2 (`WidgetLayoutLibrary.GetMousePositionOnPlatform`))
    (`PrimitiveComponent.AddImpulse` (`/Game/FunfairElements/ChambouleTout/BP_Ball.Sphere` _returnvalue) (* (`.WorldDirection` (`GameplayStatics.DeprojectScreenToWorld` (`GameplayStatics.GetPlayerController` 0) (`KismetMathLibrary.MakeVector2D` (+ (`KismetMathLibrary.BreakVector2D` _returnvalue_2) (`KismetMathLibrary.RandomFloatInRange` 0.0 _cursordist)) (+ (`.Y` (`KismetMathLibrary.BreakVector2D` _returnvalue_2)) (`KismetMathLibrary.RandomFloatInRange` 0.0 _cursordist))))) 200.0) "None" false)
    (`self.EndThrow`)))

(event `EndThrow`
  (bind _ui (`self.UI`))
  (bind _result (`/Engine/EditorBlueprintResources/StandardMacros.DecrementInt` (`self.Throw`))
    (:`  `
      (set `self.Throw` _result)
      (`self.SetUiVisibility` false)
      (`/Game/FunfairElements/ChambouleTout/WB_ChambouleTout.RemoveThrow` _ui)
      (`/Game/FunfairElements/ChambouleTout/WB_ChambouleTout.StopAnim` _ui)
      (`KismetSystemLibrary.Delay` 1.0)
      (if (and (> (`self.Throw`) 0) (< (`self.Score`) 15))
        (set `self.CanThrow` true)
        (set `self.MiniGameTime` true)
        (`self.SetUiVisibility` true)
        (`/Game/ThirdPerson/Blueprints/BP_ThirdPersonCharacter.SetCrosshairVisibility` (`self.Player`) true)
        (else
          (`/Game/ThirdPerson/Blueprints/BP_ThirdPersonCharacter.ShowWinUi` (`self.Player`) (`self.Win`) "Chamboule-tout" self))))))

(event `self.CanCheck.OnComponentEndOverlap`
  (params (OverlappedComponent :type "PrimitiveComponent Object Reference") (OtherActor :type "Actor Object Reference") (OtherComp :type "PrimitiveComponent Object Reference") (OtherBodyIndex :type Integer))
  (if (`KismetArrayLibrary.Array_Contains` (`self.AllCans`) OtherComp)
    (bind _result (`/Engine/EditorBlueprintResources/StandardMacros.IncrementInt` (`self.Score`))
      (:`  `
        (bind _output_get (set `self.Score` _result))
        (set `self.Win` (>= _output_get 8))
        (`/Game/FunfairElements/ChambouleTout/WB_ChambouleTout.AddScore` (`self.UI`))))))

(event `Replay`
  (`self.DestroyBalls`)
  (`self.ResetCanTransform`)
  (set `self.CanThrow` false)
  (set `self.Win` false)
  (set `self.Score` 0)
  (`self.StartGame`))

(fn `UserConstructionScript`)