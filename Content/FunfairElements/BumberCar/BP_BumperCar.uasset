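; BP_BumperCar is a drivable funfair bumper car pawn that the player climbs into and steers.
; PossesCar calls the player's Drive, disables its capsule collision, snaps it to the Seat socket and hands player controller 0 to the car.
; Enhanced Input rotates the spring arm to look, yaws the car directly to steer and applies forward force to move.
; A Bump event applies a supplied impulse at the hit location.
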(event `PossesCar`
  (params (Player :type "/Game/ThirdPerson/Blueprints/BP_ThirdPersonCharacter Object Reference"))
  (bind _capsulecomponent (`Character.CapsuleComponent` Player))
  (`/Game/ThirdPerson/Blueprints/BP_ThirdPersonCharacter.Drive` Player)
  (`PrimitiveComponent.SetCollisionEnabled` _capsulecomponent "NoCollision")
  (`SceneComponent.K2_AttachToComponent` _capsulecomponent (`self.Car`) "Seat" "SnapToTarget" "SnapToTarget" "KeepRelative" true)
  (`Controller.Possess` (`GameplayStatics.GetPlayerController` 0) self))

(event `Bump`
  (params (NormalImpluse :type "Vector Structure") (HitLocation :type "Vector Structure"))
  (`PrimitiveComponent.AddImpulseAtLocation` (`self.Car`) NormalImpluse HitLocation "None")
  (`KismetSystemLibrary.PrintString` "Bumped"))

(event `EnhancedInput|/Game/ThirdPerson/Input/Actions/IA_Look`
  (params (ActionValue :type "Vector2D Structure") (ElapsedSeconds :type "Float (double-precision)") (TriggeredSeconds :type "Float (double-precision)") (InputAction :type "InputAction Object Reference" :default "/Game/ThirdPerson/Input/Actions/IA_Look.IA_Look"))
  (bind _springarm (`self.SpringArm`))
  (bind (_returnvalue_roll _returnvalue_pitch _returnvalue_yaw) (`KismetMathLibrary.BreakRotator` (`SceneComponent.K2_GetComponentRotation` _springarm)))
  (:`Triggered`
    (`SceneComponent.K2_SetWorldRotation` _springarm (`KismetMathLibrary.MakeRotator` 0.0 (- _returnvalue_pitch ActionValue_Y) (+ ActionValue_X _returnvalue_yaw)) false false)))

(event `EnhancedInput|/Game/ThirdPerson/Input/Actions/IA_Move`
  (params (ActionValue :type "Vector2D Structure") (ElapsedSeconds :type "Float (double-precision)") (TriggeredSeconds :type "Float (double-precision)") (InputAction :type "InputAction Object Reference" :default "/Game/ThirdPerson/Input/Actions/IA_Move.IA_Move"))
  (bind _car (`self.Car`))
  (:`Triggered`
    (`SceneComponent.K2_AddWorldRotation` _car (`KismetMathLibrary.MakeRotator` 0.0 0.0 (* ActionValue_X 1.5)) false false)
    (`PrimitiveComponent.AddForce` _car (* (* (`SceneComponent.GetForwardVector` _car) (* ActionValue_Y 15.0)) 30000.0) "None" false)))

(fn `UserConstructionScript`)