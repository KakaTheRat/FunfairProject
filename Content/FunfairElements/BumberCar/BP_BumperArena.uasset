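; Bumper car arena minigame that seats the player in a random BP_BumperCar when they overlap the cylinder trigger.
; It starts a timed round via the WB_Bumper widget and toggles physics and movement on all cars.
; Cars leaving the box are counted and hidden; the player's exit forces a loss, otherwise knocking out half the rivals wins.
; Replay and Exit restore cached car transforms, with Exit also repossessing the character at the exit point.
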(event `self.ReceiveBeginPlay`
  (bind _outactors (`GameplayStatics.GetAllActorsOfClass` "/Game/FunfairElements/BumberCar/BP_BumperCar.BP_BumperCar_C"))
  (bind _output_get (set `self.Cars` _outactors))
  (for _array_element _output_get
    (`KismetArrayLibrary.Array_Add` (`self.InitTransform`) (`SceneComponent.K2_GetComponentToWorld` (`/Game/FunfairElements/BumberCar/BP_BumperCar.Car` _array_element)))
    (`self.CreateUI`)))

(event `self.Cylinder.OnComponentBeginOverlap`
  (params (OverlappedComponent :type "PrimitiveComponent Object Reference") (OtherActor :type "Actor Object Reference") (OtherComp :type "PrimitiveComponent Object Reference") (OtherBodyIndex :type Integer) (bFromSweep :type Boolean) (SweepResult :type "HitResult Structure (by ref)"))
  (bind _outitem (`KismetArrayLibrary.Array_Random` (`self.Cars`)))
  (bind _asbp_third_person_character (cast `/Game/ThirdPerson/Blueprints/BP_ThirdPersonCharacter` OtherActor))
  (bind _output_get (set `self.PlayerCar` _outitem))
  (bind _output_get_2 (set `self.Player` _asbp_third_person_character))
  (`/Game/FunfairElements/BumberCar/BP_BumperCar.PossesCar` _outitem _output_get_2)
  (`/Game/FunfairElements/BumberCar/BP_BumperCar.PossesCar` _output_get _output_get_2)
  (`self.StartGame`))

(event `self.Box_E9DE468F.OnComponentEndOverlap`
  (params (OverlappedComponent :type "PrimitiveComponent Object Reference") (OtherActor :type "Actor Object Reference") (OtherComp :type "PrimitiveComponent Object Reference") (OtherBodyIndex :type Integer))
  (if (`self.GameOn`)
    (if (== OtherActor (`self.PlayerCar`))
      (set `self.ForceLoose` true)
      (`self.EndGame`)
      (else
        (bind _result (`/Engine/EditorBlueprintResources/StandardMacros.IncrementInt` (`self.CarOut`))
          (:`  `
            (set `self.CarOut` _result)
            (`/Game/FunfairElements/BumberCar/WB_Bumper.CarLoose` (`self.UI`))
            (`SceneComponent.SetHiddenInGame` OtherComp true false)))))))

(event `StartGame`
  (`self.LockCars` false)
  (set `self.GameOn` true)
  (`/Game/FunfairElements/BumberCar/WB_Bumper.StartGame` (`self.UI`) 15.0 (- (`KismetArrayLibrary.Array_Length` (`self.Cars`)) 1))
  (`self.SetUIVisibility` true)
  (`self.CanMoove` true)
  (set `self.ForceLoose` false))

(event `EndGame`
  (`self.LockCars` true)
  (set `self.GameOn` true)
  (set `self.Win` (>= (`self.CarOut`) (/ (- (`KismetArrayLibrary.Array_Length` (`self.Cars`)) 1) 2)))
  (`self.CanMoove` false)
  (`self.SetUIVisibility` false)
  (bind _returnvalue (`GameplayStatics.GetActorOfClass` "/Game/ThirdPerson/Blueprints/BP_ThirdPersonCharacter.BP_ThirdPersonCharacter_C"))
  (if (`self.ForceLoose`)
    (set `self.Win` false))
  (`/Game/ThirdPerson/Blueprints/BP_ThirdPersonCharacter.ShowWinUi` _returnvalue (`self.Win`) "Auto-tamponneuse" self))

(event `Exit`
  (bind _player (`self.Player`))
  (bind _capsulecomponent (`Character.CapsuleComponent` _player))
  (`/Game/FunfairElements/BumberCar/WB_Bumper.Reset` (`self.UI`))
  (`self.ResetCars`)
  (`SceneComponent.K2_DetachFromComponent` _capsulecomponent "KeepRelative" "KeepRelative" "KeepRelative" true)
  (`Controller.Possess` (`GameplayStatics.GetPlayerController` 0) _player)
  (`SceneComponent.K2_SetWorldLocation` _capsulecomponent (+ (`SceneComponent.K2_GetComponentLocation` (`self.ExitPoint_0`)) (0.0 0.0 90.0)) false false)
  (`PrimitiveComponent.SetCollisionEnabled` _capsulecomponent "QueryAndPhysics")
  (`/Game/ThirdPerson/Blueprints/BP_ThirdPersonCharacter.Drive` (`self.Player`) false))

(event `Replay`
  (`/Game/FunfairElements/BumberCar/WB_Bumper.Reset` (`self.UI`))
  (`self.ResetCars`)
  (`self.StartGame`))

(event `CreateUI`
  (bind _returnvalue (`|CreateWidget` "/Game/FunfairElements/BumberCar/WB_Bumper.WB_Bumper_C" (`GameplayStatics.GetPlayerController` 0)))
  (set `self.UI` _returnvalue))

(event `SetUIVisibility`
  (params (visible :type Boolean))
  (bind _ui (`self.UI`))
  (if visible
    (`UserWidget.AddToViewport` _ui 0)
    (else
      (`Widget.RemoveFromParent` _ui))))

(event `ResetCars`
  (for (_array_element _array_index) (`self.Cars`)
    (bind _car (`/Game/FunfairElements/BumberCar/BP_BumperCar.Car` _array_element))
    (`SceneComponent.K2_SetWorldTransform` _car (`|GetArrayItem` (`self.InitTransform`) _array_index) false true)
    (`SceneComponent.SetHiddenInGame` _car false false)
    (`PrimitiveComponent.SetCollisionEnabled` _car "QueryAndPhysics")))

(event `CanMoove`
  (params (CanMoove :type Boolean))
  (for _array_element (`self.Cars`)
    (`/Game/FunfairElements/BumberCar/BP_BumperCar.ChangeCanMove` _array_element CanMoove)))

(event `LockCars`
  (params (`Lock?` :type Boolean))
  (for _array_element (`self.Cars`)
    (`PrimitiveComponent.SetSimulatePhysics` (`/Game/FunfairElements/BumberCar/BP_BumperCar.Car` _array_element) (not `Lock?`))))

(fn `UserConstructionScript`)